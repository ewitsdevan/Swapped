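; MovingTarget_BP is a target actor that shuttles back and forth until its Hit event fires.
; On BeginPlay it stores its location as StartLocation, then lerps its relative location toward EndLocation without sweeping.
; Two timelines alternate in an endless loop: Move plays forward, then MoveReverse plays backward and restarts Move when finished.
; The Hit event plays a 2D robot sound and destroys the actor.
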(event EventBeginPlay
  (Variables|Default|SetstartLocation (Transformation|GetActorLocation))
  (bind _move (Timeline|Move PlayFromStart)
    (:Update
      (Transformation|SetActorRelativeLocation (Math|Vector|Lerp(Vector) (Variables|Default|GetstartLocation) (Variables|Default|GetendLocation) _move)))
    (:Finished
      (bind _move_2 (Timeline|Move%20Reverse ReverseFromEnd)
        (:Update
          (Transformation|SetActorRelativeLocation (Math|Vector|Lerp(Vector) (Variables|Default|GetstartLocation) (Variables|Default|GetendLocation) _move_2)))
        (:Finished
          (Timeline|Move PlayFromStart))))))

(event Collision|EventHit
  (params (MyComp :type Primitive%20Component%20Object%20Reference) (Other :type Actor%20Object%20Reference) (OtherComp :type Primitive%20Component%20Object%20Reference) (bSelfMoved :type Boolean) (HitLocation :type Vector :default "0, 0, 0") (HitNormal :type Vector :default "0, 0, 0") (NormalImpulse :type Vector :default "0, 0, 0") (Hit :type Hit%20Result%20Structure%20%28by%20ref%29))
  (Audio|PlaySound2D "/Game/Audio/Robot_SW.Robot_SW" 2.0 1.0 0.0 0 0)
  (Actor|DestroyActor))

(fn ConstructionScript)